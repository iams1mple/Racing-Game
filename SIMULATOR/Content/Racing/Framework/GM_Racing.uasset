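; Racing game mode that runs a checkpoint time-trial: a delayed start, a countdown timer, and a win or lose result printed on screen.
; On BeginPlay it binds to every BP_checkPoint, separating the finish from time-awarding checkpoints.
; Added time restarts the timer with remaining plus bonus seconds and plays a HUD animation.
; Timer expiry triggers Lose, while crossing the finish clears the timer and wins.
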(event `self.ReceiveBeginPlay`
  (`|ExecutionSequence`
    (:`then_0`
      (bind _outactors (`GameplayStatics.GetAllActorsOfClass` "/Game/Racing/Checkpoint/BP_checkPoint.BP_checkPoint_C"))
      (for _array_element _outactors
        (if (`/Game/Racing/Checkpoint/BP_checkPoint.IsFinish` _array_element)
          (add `/Game/Racing/Checkpoint/BP_checkPoint.CheckPointCrossed` _array_element (`|CreateDelegate` :!event `Win_CrossFinishLine`))
          (else
            (add `/Game/Racing/Checkpoint/BP_checkPoint.CheckPointCrossedWithTime` _array_element (`|CreateDelegate` :!event `CrossedACheckpoint`))))))
    (:`then_1`
      (`self.Start countdown`))))

(event `Start countdown`
  (`KismetSystemLibrary.Delay` 1.0)
  (`KismetSystemLibrary.PrintString` "Game Start")
  (`KismetSystemLibrary.Delay` (`self.StartCountdownDuration`))
  (`self.Start`))

(event `Start`
  (`KismetSystemLibrary.PrintString` "Pedal")
  (bind _returnvalue (`KismetSystemLibrary.K2_SetTimerDelegate` (delegate `Lose`) (`self.StartTimeDuration`)))
  (set `self.TimeRemainingTimer` _returnvalue))

(event `Lose`
  (`self.End` false))

(event `Win_CrossFinishLine`
  (`KismetSystemLibrary.K2_ClearAndInvalidateTimerHandle` (`self.TimeRemainingTimer`))
  (`self.End` true))

(event `End`
  (params (win :type Boolean))
  (`KismetSystemLibrary.PrintString` (`KismetMathLibrary.SelectString` "You win" "You lose" win)))

(event `CrossedACheckpoint`
  (params (TimeToAdd :type Integer))
  (`self.AddTimerToTime` TimeToAdd))

(fn `AddTimerToTime`
  (params (TimeToAdd :type Integer))
  (bind _returnvalue (`KismetSystemLibrary.K2_SetTimerDelegate` (`|CreateDelegate` :!event `Lose`) (+ (`KismetSystemLibrary.K2_GetTimerRemainingTimeHandle` (`self.TimeRemainingTimer`)) (`local.TimeToAdd`))))
  (set `self.TimeRemainingTimer` _returnvalue)
  (bind _asvehicle_player_controller (cast `/Game/VehicleTemplate/Blueprints/VehiclePlayerController` (`GameplayStatics.GetPlayerController` 0)))
  (`/Game/VehicleTemplate/Blueprints/VehicleUI.PlayAnimationTimeAdded` (`/Game/VehicleTemplate/Blueprints/VehiclePlayerController.VehicleHud` _asvehicle_player_controller)))

(fn `UserConstructionScript`)